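; BP_SM_P38 is a P-38 aircraft Blueprint that animates its two spinning propellers.
; Each Tick calls the SMP38 function, which multiplies world delta seconds by Speed for a frame-rate-independent roll increment.
; The function applies that same local rotation to RightPropeller and LeftPropeller, so both turn in the same direction.
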(event Collision|EventActorBeginOverlap
  (params (OtherActor :type Actor%20Object%20Reference)))

(event EventTick
  (params (DeltaSeconds :type Float%20%28single-precision%29))
  (CallFunction|SMP38))

(fn ConstructionScript)

(fn SMP38
  (bind _output_get (Variables|Default|SetMoter (* (Utilities|Time|GetWorldDeltaSeconds) (Variables|Default|GetSpeed))))
  (Transformation|AddLocalRotation (Variables|Default|GetRight_Propeller) (Math|Rotator|MakeRotator _output_get 0.0 0.0) false false)
  (Transformation|AddLocalRotation (Variables|Default|GetLeft_Propeller) (Math|Rotator|MakeRotator (Variables|Default|GetMoter) 0.0 0.0) false false))